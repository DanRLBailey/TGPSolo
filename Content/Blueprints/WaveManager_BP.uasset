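; Wave manager Blueprint that tracks enemy wave progression and the score.
; Every Tick it recomputes Score as CurrentWave plus EnemiesKilled and polls for live EnemyBase_BP actors.
; When none remain and WaveCount equals CurrentWave, it increments the wave and resets WaveCount.
; SpawnEnemy, commented "C++ This", prints the wave number and calls CallSpawnEnemy0; nothing here triggers it or increments WaveCount.
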(event Custom|IncreaseWave
  (Variables|Default|SetcurrentWave (+ (Variables|Default|GetcurrentWave) 1))
  (Variables|Default|SetwaveCount 0))

(event Custom|GetScore
  (Variables|Default|Setscore (+ (Variables|Default|GetcurrentWave) (Variables|Default|GetenemiesKilled))))

(event EventSpawnEnemy
  ;[1 1 1] C++ This
  (Development|PrintString (Utilities|String|ToString(Integer) (Variables|Default|GetcurrentWave)))
  (Default|CallSpawnEnemy0))

(event EventTick
  (params (DeltaSeconds :type Float%20%28single-precision%29))
  (CallFunction|GetScore)
  (bind _outactors (Actor|GetAllActorsOfClass "/Game/Blueprints/EnemyBase_BP.EnemyBase_BP_C"))
  (if (<= (Utilities|Array|Length _outactors) 0)
    (if (== (Variables|Default|GetwaveCount) (Variables|Default|GetcurrentWave))
      (CallFunction|IncreaseWave))))

(fn ConstructionScript)