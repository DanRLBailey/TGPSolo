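; Base rocket actor that explodes on contact with an enemy and deals area damage.
; A sphere collision maintains the list of overlapping enemies and players, identified by interface checks.
; Explode and ExplodeBP share one path: spawn an explosion emitter, send two damage messages of differing strength to each listed actor, then destroy the rocket.
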(event OnComponentBeginOverlap(RocketCollision)
  (params (OverlappedComponent :type Primitive%20Component%20Object%20Reference) (OtherActor :type Actor%20Object%20Reference) (OtherComp :type Primitive%20Component%20Object%20Reference) (OtherBodyIndex :type Integer) (bFromSweep :type Boolean) (SweepResult :type Hit%20Result%20Structure%20%28by%20ref%29))
  (if (Utilities|DoesObjectImplementInterface OtherActor "/Game/Blueprints/IIsEnemy.IIsEnemy_C")
    (CallFunction|ExplodeBP)))

(event OnComponentBeginOverlap(SphereCollision)
  (params (OverlappedComponent :type Primitive%20Component%20Object%20Reference) (OtherActor :type Actor%20Object%20Reference) (OtherComp :type Primitive%20Component%20Object%20Reference) (OtherBodyIndex :type Integer) (bFromSweep :type Boolean) (SweepResult :type Hit%20Result%20Structure%20%28by%20ref%29))
  (if (or (Utilities|DoesObjectImplementInterface OtherActor "/Game/Blueprints/IIsEnemy.IIsEnemy_C") (Utilities|DoesObjectImplementInterface OtherActor "/Game/Blueprints/IIsPlayer.IIsPlayer_C"))
    (Utilities|Array|Add (Variables|Default|GetAffected%20Actors) OtherActor)))

(event OnComponentEndOverlap(SphereCollision)
  (params (OverlappedComponent :type Primitive%20Component%20Object%20Reference) (OtherActor :type Actor%20Object%20Reference) (OtherComp :type Primitive%20Component%20Object%20Reference) (OtherBodyIndex :type Integer))
  (Utilities|Array|RemoveItem (Variables|Default|GetAffected%20Actors) OtherActor))

(event Custom|ExplodeBP
  (Effects|SpawnEmitteratLocation "/Game/StarterContent/Particles/P_Explosion.P_Explosion" (Transformation|GetActorLocation) "0, 0, 0" "2.000000,2.000000,2.000000")
  (for _array_element (Variables|Default|GetAffected%20Actors)
    (Class|IIsEnemy|Damage(Message) _array_element 1.0)
    (Class|IIsPlayer|Damage(Message) _array_element 0.5))
  (Actor|DestroyActor))

(event EventBeginPlay)

(event Collision|EventActorBeginOverlap
  (params (OtherActor :type Actor%20Object%20Reference)))

(event EventTick
  (params (DeltaSeconds :type Float%20%28single-precision%29)))

(event EventExplode
  (Effects|SpawnEmitteratLocation "/Game/StarterContent/Particles/P_Explosion.P_Explosion" (Transformation|GetActorLocation) "0, 0, 0" "2.000000,2.000000,2.000000")
  (for _array_element (Variables|Default|GetAffected%20Actors)
    (Class|IIsEnemy|Damage(Message) _array_element 1.0)
    (Class|IIsPlayer|Damage(Message) _array_element 0.5))
  (Actor|DestroyActor))

(fn ConstructionScript)