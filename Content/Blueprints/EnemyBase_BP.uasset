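; Base enemy Blueprint that chases and shoots the player while the player's Health is at least zero.
; It caches the player on BeginPlay, and MovetoPlayer turns toward the player and nudges forward by a fixed local offset without sweep.
; FireWeapon spawns an EnemyBulletBase_BP at its own transform and Damage subtracts Health.
; OnDeath destroys the enemy and increments EnemiesKilled on the first WaveManager_BP found.
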(event EventOnDeath
  (Actor|DestroyActor)
  (bind _outactors (Actor|GetAllActorsOfClass "/Game/Blueprints/WaveManager_BP.WaveManager_BP_C"))
  (Variables|/Script/TGPSolo.WaveManager|SetenemiesKilled (Utilities|Array|Get(acopy) _outactors) (+ (Variables|/Script/TGPSolo.WaveManager|GetenemiesKilled (Utilities|Array|Get(acopy) _outactors)) 1)))

(event EventMovetoPlayer
  (bind _returnvalue (Transformation|GetActorLocation))
  (bind _returnvalue_2 (Game|Player|GetPlayerPawn 0))
  (bind _returnvalue_3 (Transformation|GetActorLocation _returnvalue_2))
  (bind _returnvalue_4 (Math|Rotator|FindLookatRotation _returnvalue _returnvalue_3))
  (if (>= (Variables|/Script/TGPSolo.PlayerCharacter|Gethealth (Variables|Default|GetPlayerCharacter)) 0.0)
    (Transformation|SetActorRotation (Math|Rotator|MakeRotator (.roll _returnvalue_4) 0.0 (.yaw _returnvalue_4)))
    (Transformation|AddActorLocalOffset "2.000000, 0, 0" false false)))

(event EventDamage
  (params (DamageValue :type Float%20%28single-precision%29))
  (Variables|Default|Sethealth (- (Variables|Default|Gethealth) DamageValue)))

(event EventFireWeapon
  (if (>= (Variables|/Script/TGPSolo.PlayerCharacter|Gethealth (Variables|Default|GetPlayerCharacter)) 0.0)
    (Game|SpawnActorfromClass "/Game/Blueprints/EnemyBulletBase_BP.EnemyBulletBase_BP_C" (Transformation|GetActorTransform) "Undefined" 0 0)))

(event EventBeginPlay
  (bind _asplayer_character_bp (Utilities|Casting|CastToPlayerCharacter_BP (Game|Player|GetPlayerPawn 0)))
  (Variables|Default|SetPlayerCharacter _asplayer_character_bp))

(fn ConstructionScript)