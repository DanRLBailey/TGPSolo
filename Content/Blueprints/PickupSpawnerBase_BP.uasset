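; Base pickup spawner actor that spawns a health pickup at its own transform when SpawnPickup is called.
; A Box component's begin and end overlaps with Pickup_Health actors set and clear a HasHealth flag.
; SpawnPickup spawns only while that flag is false, so it avoids stacking a pickup where one already sits.
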(event OnComponentBeginOverlap(Box)
  (params (OverlappedComponent :type Primitive%20Component%20Object%20Reference) (OtherActor :type Actor%20Object%20Reference) (OtherComp :type Primitive%20Component%20Object%20Reference) (OtherBodyIndex :type Integer) (bFromSweep :type Boolean) (SweepResult :type Hit%20Result%20Structure%20%28by%20ref%29))
  (if (== (Utilities|GetClass OtherActor) "/Game/Blueprints/Pickup_Health.Pickup_Health_C")
    (Variables|Default|SetHasHealth true)))

(event OnComponentEndOverlap(Box)
  (params (OverlappedComponent :type Primitive%20Component%20Object%20Reference) (OtherActor :type Actor%20Object%20Reference) (OtherComp :type Primitive%20Component%20Object%20Reference) (OtherBodyIndex :type Integer))
  (if (== (Utilities|GetClass OtherActor) "/Game/Blueprints/Pickup_Health.Pickup_Health_C")
    (Variables|Default|SetHasHealth false)))

(event EventBeginPlay)

(event Collision|EventActorBeginOverlap
  (params (OtherActor :type Actor%20Object%20Reference)))

(event EventTick
  (params (DeltaSeconds :type Float%20%28single-precision%29)))

(event EventSpawnPickup
  (if (not (Variables|Default|GetHasHealth))
    (Game|SpawnActorfromClass "/Game/Blueprints/Pickup_Health.Pickup_Health_C" (Transformation|GetActorTransform) "Undefined" 0 0)))

(fn ConstructionScript)