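; Base bomb actor that is lobbed forward and up on spawn and damages nearby players and enemies when it explodes.
; BeginPlay offsets the mesh and applies an impulse in the actor's local frame.
; Collision overlaps maintain a list of affected actors implementing the enemy or player interface.
; The Explode event, not triggered within this Blueprint, spawns an explosion particle and sends two damage messages to each listed actor.
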(event OnComponentBeginOverlap(Collision)
  (params (OverlappedComponent :type Primitive%20Component%20Object%20Reference) (OtherActor :type Actor%20Object%20Reference) (OtherComp :type Primitive%20Component%20Object%20Reference) (OtherBodyIndex :type Integer) (bFromSweep :type Boolean) (SweepResult :type Hit%20Result%20Structure%20%28by%20ref%29))
  (if (or (Utilities|DoesObjectImplementInterface OtherActor "/Game/Blueprints/IIsEnemy.IIsEnemy_C") (Utilities|DoesObjectImplementInterface OtherActor "/Game/Blueprints/IIsPlayer.IIsPlayer_C"))
    (Utilities|Array|Add (Variables|Default|GetAffectedActors) OtherActor)))

(event OnComponentEndOverlap(Collision)
  (params (OverlappedComponent :type Primitive%20Component%20Object%20Reference) (OtherActor :type Actor%20Object%20Reference) (OtherComp :type Primitive%20Component%20Object%20Reference) (OtherBodyIndex :type Integer))
  (Utilities|Array|RemoveItem (Variables|Default|GetAffectedActors) OtherActor))

(event EventBeginPlay
  (bind _mesh (Variables|Character|GetMesh))
  (Transformation|AddLocalOffset _mesh "100.000000,0.000000,0.000000" false false)
  (Physics|AddImpulse _mesh (Math|Transform|TransformDirection (Transformation|GetActorTransform self) "50000.000000, 0,75000.000000") "None" false))

(event Collision|EventActorBeginOverlap
  (params (OtherActor :type Actor%20Object%20Reference)))

(event EventTick
  (params (DeltaSeconds :type Float%20%28single-precision%29)))

(event EventExplode
  (Effects|SpawnEmitteratLocation "/Game/StarterContent/Particles/P_Explosion.P_Explosion" (Transformation|GetActorLocation) "0, 0, 0" "2.000000,2.000000,2.000000")
  (for _array_element (Variables|Default|GetAffectedActors)
    (Class|IIsEnemy|Damage(Message) _array_element 1.0)
    (Class|IIsPlayer|Damage(Message) _array_element 0.5)))

(fn ConstructionScript)