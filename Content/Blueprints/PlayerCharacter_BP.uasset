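; Player character that aims at the mouse cursor, spawns a bomb on Fire input and loses Health on damage.
; Tick drives ChangeWeapon, which picks a random weapon index after a random delay, and calls FireWeapon, which is empty.
; A disconnected chain, never run, holds delayed firing by weapon: single, three-way shotgun with recoil impulse on Ball, one-at-a-time laser, or bomb.
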(event Custom|ChangeWeapon
  (Utilities|FlowControl|Delay (Math|Random|RandomFloatinRange 3.0 7.0))
  (Variables|Default|SetcurrentWeapon (Math|Random|RandomIntegerinRange 0 (- (Utilities|Array|Length (Variables|Default|GetweaponArray)) 1))))

(event Custom|FireWeapon)

(event EventBeginPlay
  (Variables|/Script/Engine.PlayerController|SetbShowMouseCursor (Game|GetPlayerController 0) true))

(event Collision|EventActorBeginOverlap
  (params (OtherActor :type Actor%20Object%20Reference)))

(event EventTick
  (params (DeltaSeconds :type Float%20%28single-precision%29))
  (CallFunction|ChangeWeapon)
  (CallFunction|FireWeapon))

(event EventDamage
  (params (DamageValue :type Float%20%28single-precision%29))
  (Variables|Default|Sethealth (- (Variables|Default|Gethealth) DamageValue)))

(event Input|ActionEvents|InputActionFire
  (params (Key :type Key%20Structure))
  (bind _returnvalue (Game|Player|GetPlayerPawn 0))
  (bind _returnvalue_2 (Game|GetPlayerController 0))
  (bind _returnvalue_3 (Transformation|GetActorLocation _returnvalue))
  (bind _hitresult (Game|Player|GetHitResultUnderCursorbyChannel _returnvalue_2 "TraceTypeQuery1" true))
  (bind _returnvalue_4 (Math|Rotator|FindLookatRotation _returnvalue_3 (.location _hitresult)))
  (:Pressed
    (Development|PrintString "Bomb")
    (Game|SpawnActorfromClass "/Game/Blueprints/BombBase_BP.BombBase_BP_C" (Math|Transform|MakeTransform _returnvalue_3 (Math|Rotator|MakeRotator (.roll _returnvalue_4) 0.0 (.yaw _returnvalue_4))) "Undefined" 0 0)))

(fn ConstructionScript)